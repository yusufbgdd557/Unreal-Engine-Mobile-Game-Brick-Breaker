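; MainPlayer is the touch-controlled paddle of a brick-breaker game, which also handles level win and loss.
; On BeginPlay it spawns a Ball_BP at its Arrow, then polls the Brick_BP count on a delay loop and opens the next level at zero.
; While touched, Tick moves the Player component along Y to the traced finger hit.
; A ball overlapping DeathCollusion dies, and the current level reloads after a delay.
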(event OnComponentBeginOverlap(DeathCollusion)
  (params (OverlappedComponent :type Primitive%20Component%20Object%20Reference) (OtherActor :type Actor%20Object%20Reference) (OtherComp :type Primitive%20Component%20Object%20Reference) (OtherBodyIndex :type Integer) (bFromSweep :type Boolean) (SweepResult :type Hit%20Result%20Structure%20%28by%20ref%29))
  (bind _asball_bp (Utilities|Casting|CastToBall_BP OtherActor))
  (Default|Death _asball_bp)
  (Utilities|FlowControl|Delay 3.0)
  (bind _returnvalue (Game|GetCurrentLevelName true))
  (Game|OpenLevel(byName) (Utilities|String|StringToName _returnvalue)))

(event EventBeginPlay
  (bind _arrow (Variables|Default|GetArrow))
  (bind _returnvalue (Transformation|GetWorldTransform _arrow))
  (Game|SpawnActorfromClass "/Game/Blueprints/Ball_BP.Ball_BP_C" (Math|Transform|MakeTransform (Math|Vector|MakeVector (.x (.location _returnvalue)) (.y (.location _returnvalue)) 1e+02) "0, 0, 0" "1,1,1") "Undefined" 0 0)
  (bind _outactors (Actor|GetAllActorsOfClass "/Game/Blueprints/Brick_BP.Brick_BP_C" :!label _label))
  (if (== (Utilities|Array|Length _outactors) 0)
    (Game|OpenLevel(byName) (Variables|Default|GetNextLevel))
    (else
      (Development|PrintString (Utilities|String|ToString(Integer) (Utilities|Array|Length _outactors)))
      (Utilities|FlowControl|Delay 3.0)
      (goto _label))))

(event EventTick
  (params (DeltaSeconds :type Float%20%28single-precision%29))
  (bind _player (Variables|Default|GetPlayer))
  (bind _player_2 (Variables|Default|GetPlayer))
  (if (Variables|Default|GetIsTouching)
    ;[1 1 1] If finger is on screen
    (Transformation|SetWorldLocation _player_2 (Math|Vector|MakeVector (.x (Transformation|GetWorldLocation _player_2)) (.Y (Math|Vector|BreakVector (.location (.HitResult (Class|PlayerController|GetHitResultUnderFingerbyChannel (Game|GetPlayerController 0) "Touch1" "TraceTypeQuery1" true))))) 1e+02) false false)
    (else
      ;[1 1 1] If finger is NOT on screen
      (Transformation|SetWorldLocation _player (Transformation|GetWorldLocation _player) false false))))

(event Input|TouchEvents|InputTouch
  (params (Location :type Vector) (FingerIndex :type ETouchIndex%20Enum))
  (:Pressed
    (Variables|Default|SetIsTouching true))
  (:Released
    (Variables|Default|SetIsTouching false)))

(fn ConstructionScript)