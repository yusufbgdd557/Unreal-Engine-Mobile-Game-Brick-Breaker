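; Ball actor Blueprint that launches a physics ball at level start and handles its death.
; BeginPlay sets the Sphere's height, keeping its X and Y, then applies a one-time impulse along Y.
; The Death event shows a GameOver widget, waits briefly, then reloads the current level by name.
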(event Custom|Death
  (bind _returnvalue (UserInterface|CreateWidget "/Game/Widgets/GameOver.GameOver_C"))
  (UserInterface|Viewport|AddtoViewport _returnvalue 0)
  (Utilities|FlowControl|Delay 3.0)
  (bind _returnvalue_2 (Game|GetCurrentLevelName true))
  (Game|OpenLevel(byName) (Utilities|String|StringToName _returnvalue_2)))

(event EventBeginPlay
  (bind _sphere (Variables|Default|GetSphere))
  (bind _returnvalue (Transformation|GetWorldLocation _sphere))
  (Transformation|SetWorldLocation _sphere (Math|Vector|MakeVector (.x _returnvalue) (.y _returnvalue) 1e+02) false false)
  (Physics|AddImpulse _sphere (Math|Vector|MakeVector 0.0 (* 1e+03 75.0) 0.0) "None" false))

(fn ConstructionScript)